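; Door actor that fades away and destroys itself once its RemainingActors list is empty.
; CheckRemainingActors triggers OpenDoor, which requires a valid Camera, blends the player view to it and plays a sound.
; The OpenTime timeline drives Opacity on a dynamic material instance of the mesh, then destroys the door and blends the view back to the controlled pawn.
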(event Custom|OpenDoor
  (bind _returnvalue (Game|GetPlayerController 0))
  (bind _camera (Variables|Default|GetCamera))
  (Utilities|IsValid _camera
    (:Is%20Valid
      (Game|Player|SetViewTargetwithBlend (Game|GetPlayerController 0) _camera 1.5 "VTBlend_Cubic" 0.0 false)
      ;[1 1 1] Alpha channel of the door to 0
      (bind _returnvalue_2 (Rendering|Material|CreateDynamicMaterialInstance (Variables|Default|GetStaticMesh) 0 0 :!class /Script/Engine.PrimitiveComponent))
      (Audio|PlaySound2D "/Game/Audio/Dark_Spell__1_.Dark_Spell__1_" 0.5)
      (bind _opacity (Timeline|OpenTime PlayFromStart)
        (:Update
          (Rendering|Material|SetScalarParameterValue _returnvalue_2 "Opacity" _opacity :!class /Script/Engine.MaterialInstanceDynamic))
        (:Finished
          (Actor|DestroyActor)
          (Game|Player|SetViewTargetwithBlend _returnvalue (Pawn|GetControlledPawn _returnvalue) 1.0 "VTBlend_Cubic" 0.0 false))))))

(fn ConstructionScript)

(fn CheckRemainingActors
  (if (<= (Utilities|Array|Length (Variables|Default|GetRemainingActors)) 0)
    (CallFunction|OpenDoor)))