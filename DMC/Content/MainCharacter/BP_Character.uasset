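; Player character Blueprint handling melee combat input: defense, a five-hit basic attack combo, a focus dash and jump.
; Attack starts the combo montage, or jumps straight to its next section if already playing, looping after the fifth.
; While Focus is held, Attack calls TryDash, which needs grounded forward movement and briefly zeroes ground friction for a forward impulse.
; Defense plays its montage until released; Jump cancels the current montage.
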(event Input|ActionEvents|InputActionDefense
  (params (Key :type Key%20Structure))
  (:Pressed
    (Animation|PlayAnimMontage "/Game/MainCharacter/Animations/AM_Attacks_defence_stand_Montage.AM_Attacks_defence_stand_Montage" 1.0 "None"))
  (:Released
    (Animation|StopAnimMontage "/Game/MainCharacter/Animations/AM_Attacks_defence_stand_Montage.AM_Attacks_defence_stand_Montage")))

(event Input|ActionEvents|InputActionAttack
  (params (Key :type Key%20Structure))
  (bind _mesh (Variables|Character|GetMesh))
  (bind _returnvalue (Components|SkeletalMesh|GetAnimInstance _mesh))
  (:Pressed
    (if (Variables|Default|Getfocusing)
      (Utilities|FlowControl|Sequence
        (:then_0
          (Utilities|TryDash)))
      (elif (not (Class|AnimInstance|MontageIsActive _returnvalue "/Game/MainCharacter/Animations/AM_Basic_Attack_Montage.AM_Basic_Attack_Montage"))
        (Animation|PlayAnimMontage "/Game/MainCharacter/Animations/AM_Basic_Attack_Montage.AM_Basic_Attack_Montage" 1.0 "BasicAttack01")
        (else
          (Utilities|FlowControl|Sequence
            (:then_0
              (switch name (Animation|Montage|MontageGetCurrentSection _returnvalue "/Game/MainCharacter/Animations/AM_Basic_Attack_Montage.AM_Basic_Attack_Montage")
                (:BasicAttack01
                  (Variables|Default|SetNextMontage "BasicAttack02"))
                (:BasicAttack02
                  (Variables|Default|SetNextMontage "BasicAttack03"))
                (:BasicAttack03
                  (Variables|Default|SetNextMontage "BasicAttack04"))
                (:BasicAttack04
                  (Variables|Default|SetNextMontage "BasicAttack05"))
                (:BasicAttack05
                  (Variables|Default|SetNextMontage "BasicAttack01"))))
            (:then_1
              (Ability|Animation|MontageJumptoSection _returnvalue (Variables|Default|GetNextMontage)))))))))

(event Input|ActionEvents|InputActionFocus
  (params (Key :type Key%20Structure))
  (:Pressed
    (Variables|Default|Setfocusing true))
  (:Released
    (Variables|Default|Setfocusing false)))

(event Input|ActionEvents|InputActionJump
  (params (Key :type Key%20Structure))
  (:Pressed
    (bind _returnvalue (Animation|GetCurrentMontage :!class /Script/Engine.Character))
    (Animation|StopAnimMontage _returnvalue)
    (Character|Jump)))

(fn ConstructionScript)

(fn GetCurrentVelocity
  (bind _output_get (Variables|Default|Setvelocity (Math|Transform|InverseTransformDirection (Transformation|GetActorTransform) (Transformation|GetVelocity))))
  (return _output_get))