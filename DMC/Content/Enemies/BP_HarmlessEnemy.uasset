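; BP_HarmlessEnemy is an enemy that takes damage and displays its health on a healthbar widget, with no attack logic in this graph.
; AnyDamage subtracts incoming damage from Health while IsDead is false and prints the new value as debug output.
; Tick pushes the raw Health value into the WBP_Healthbar's HealthFactor every frame rather than updating it when damage occurs.
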(event EventBeginPlay)

(event Collision|EventActorBeginOverlap
  (params (OtherActor :type Actor%20Object%20Reference)))

(event EventTick
  (params (DeltaSeconds :type Float%20%28single-precision%29))
  (bind _aswbp_healthbar (Utilities|Casting|CastToWBP_Healthbar (UserInterface|GetUserWidgetObject (Variables|Default|GetHealthbar))))
  (Variables|/Game/UI_Widgets/WBP_Healthbar.WBP_Healthbar_C|SetHealthFactor _aswbp_healthbar (Variables|Default|Gethealth)))

(event Game|Damage|EventAnyDamage
  (params (Damage :type Float%20%28single-precision%29) (DamageType :type Damage%20Type%20Object%20Reference) (InstigatedBy :type Controller%20Object%20Reference) (DamageCauser :type Actor%20Object%20Reference))
  (if (not (Class|DMCCharacter|IsDead))
    (bind _output_get (Variables|Default|Sethealth (- (Variables|Default|Gethealth) Damage)))
    (Development|PrintString (Utilities|String|ToString(Float) _output_get))))

(fn ConstructionScript)