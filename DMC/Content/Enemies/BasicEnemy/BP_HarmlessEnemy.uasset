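; BP_HarmlessEnemy is a basic enemy with health that can be linked to closed doors, with no attack logic in this graph.
; Tick copies Health into its healthbar widget, and AnyDamage lowers Health and plays a hit sound.
; On death it destroys the healthbar and capsule components, then removes itself from each linked door's RemainingActors and has that door recheck whether to open.
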(event EventBeginPlay)

(event Collision|EventActorBeginOverlap
  (params (OtherActor :type Actor%20Object%20Reference)))

(event EventTick
  (params (DeltaSeconds :type Float%20%28single-precision%29))
  (bind _healthbar (Variables|Default|GetHealthbar))
  (Utilities|IsValid _healthbar
    (:Is%20Valid
      (bind _aswbp_healthbar (Utilities|Casting|CastToWBP_Healthbar (UserInterface|GetUserWidgetObject _healthbar)))
      (Variables|/Game/UI_Widgets/WBP_Healthbar.WBP_Healthbar_C|SetHealthFactor _aswbp_healthbar (Variables|Default|Gethealth)))))

(event Game|Damage|EventAnyDamage
  (params (Damage :type Float%20%28single-precision%29) (DamageType :type Damage%20Type%20Object%20Reference) (InstigatedBy :type Controller%20Object%20Reference) (DamageCauser :type Actor%20Object%20Reference))
  (if (not (Class|DMCCharacter|IsDead))
    (Variables|Default|Sethealth (- (Variables|Default|Gethealth) Damage))
    (Audio|PlaySound2D "/Game/Audio/SC_Hit.SC_Hit" 0.6)
    (if (Class|DMCCharacter|IsDead)
      (Components|DestroyComponent (Variables|Default|GetHealthbar))
      (Components|DestroyComponent (Variables|Default|GetCapsuleComponent))
      (CallFunction|UnlinkDoors))))

(fn ConstructionScript)

(fn UnlinkDoors
  ;[1 1 1] Check if enemy is one of remaining actors of the linked doors, in that case remove from the door array and check if door should open
  (for _array_element (Variables|Default|GetClosedDoors)
    (bind _output_get (LocalVariables|SetBP_Door _array_element))
    (for _array_element_2 (Variables|/Game/Blueprints/BP_Door.BP_Door_C|GetRemainingActors _output_get)
      (if (== _array_element_2 self)
        (bind _returnvalue (Utilities|Array|RemoveItem (Variables|/Game/Blueprints/BP_Door.BP_Door_C|GetRemainingActors _output_get) _array_element_2))
        (if _returnvalue
          (Default|CheckRemainingActors (LocalVariables|GetBP_Door)))))))