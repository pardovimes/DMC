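; AI controller for the basic enemy that gives it the player as a target through perception.
; On BeginPlay it loads BB_BasicEnemy, caches the blackboard component and runs BT_BasicEnemy.
; When perception updates include player character 0, it writes that character to the Target key, without checking whether it was sensed or lost and without ever clearing it.
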(event OnPerceptionUpdated(AIPerception)
  (params (UpdatedActors :type Array%20of%20Actor%20Object%20References))
  (bind _returnvalue (Game|GetPlayerCharacter 0))
  (for _array_element UpdatedActors
    (if (== _array_element _returnvalue)
      (AI|Components|Blackboard|SetValueasObject (Variables|Default|GetBB_HarmlessEnemy) (Variables|Default|GetTarget) _returnvalue))))

(event EventBeginPlay
  (bind _blackboardcomponent (Class|AIController|UseBlackboard "/Game/Enemies/BasicEnemy/AI/BB_BasicEnemy.BB_BasicEnemy"))
  (Variables|Default|SetBB_HarmlessEnemy _blackboardcomponent)
  (AI|RunBehaviorTree "/Game/Enemies/BasicEnemy/AI/BT_BasicEnemy.BT_BasicEnemy"))

(fn ConstructionScript)